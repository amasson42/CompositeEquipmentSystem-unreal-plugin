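; BP_CompositeEquipmentSystem_Studio is a studio Blueprint that hosts a CompositeEquipment component to apply composite equipment to a mesh.
; The construction script initializes the component with the mesh as leader pose, then registers the Composite under CompositeName as a custom entry.
; AddKey and RemoveKey events add or remove that composite name on the component.
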(event Custom|RemoveKey
  (Class|CompositeEquipmentComponent|RemoveCompositeName (Variables|Default|GetCompositeEquipment) (Variables|Default|GetCompositeName)))

(event Custom|AddKey
  (Class|CompositeEquipmentComponent|AddCompositeName (Variables|Default|GetCompositeEquipment) (Variables|Default|GetCompositeName)))

(event EventBeginPlay)

(fn ConstructionScript
  (Class|CompositeEquipmentComponent|InitializewithLeaderPose (Variables|Default|GetCompositeEquipment) (Variables|Character|GetMesh))
  (Class|CompositeEquipmentComponent|AddCompositeCustom (Variables|Default|GetCompositeEquipment) (Variables|Default|GetComposite) (Variables|Default|GetCompositeName)))